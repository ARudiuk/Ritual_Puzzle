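; BP_Amazon_Pawn1 is a clickable board piece that the first player controller possesses on click.
; Possession lights the piece's glow, has the GridMaster get moveable tiles, and passes it the pawn's grid index, derived from its transform.
; Unpossession turns the glow off.
; The construction script creates the dynamic material for the glow and caches the first GridMaster found in the level.
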(event EventPossessed
  (params (NewController :type Controller%20Object%20Reference))
  (Rendering|Material|SetScalarParameterValue (Variables|Default|GetPawn_Material) "Glow" 1.0 :!class /Script/Engine.MaterialInstanceDynamic)
  (Default|GetMoveableTiles (Variables|Default|GetGridMaster))
  (Default|SetPossessedPawnIndex (Variables|Default|GetGridMaster) (Utilities|CoordtoIndex (Transformation|GetActorTransform self))))

(event EventUnpossessed
  (params (OldController :type Controller%20Object%20Reference))
  (Rendering|Material|SetScalarParameterValue (Variables|Default|GetPawn_Material) "Glow" 0.0 :!class /Script/Engine.MaterialInstanceDynamic))

(event MouseInput|EventActorOnClicked
  (Pawn|Possess (Game|GetPlayerController 0) self))

(event EventBeginPlay)

(event EventActorBeginOverlap
  (params (OtherActor :type Actor%20Object%20Reference)))

(event EventTick
  (params (DeltaSeconds :type Float%20%28single-precision%29)))

(fn ConstructionScript
  (bind _returnvalue (Rendering|Material|CreateDynamicMaterialInstance (Variables|Default|GetPawn) 0 "/Game/Materials/M_Amazon_Pawn1.M_Amazon_Pawn1" :!class /Script/Engine.PrimitiveComponent))
  (Variables|Default|SetPawn_Material _returnvalue)
  (bind _outactors (Actor|GetAllActorsOfClass "/Game/Blueprints/BP_Amazon_GridMaster.BP_Amazon_GridMaster_C"))
  (Variables|Default|SetGridMaster (Utilities|Array|Get(acopy) _outactors)))