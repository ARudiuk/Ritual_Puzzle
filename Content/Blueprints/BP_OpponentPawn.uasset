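; BP_OpponentPawn is the opponent's piece in a grid-based game managed by BP_Amazon_GridMaster.
; Its construction script creates and stores a dynamic instance of M_OpponentPawn and caches the first grid master found in the level.
; Coord_to_Index holds only an unused expression mapping world location to a grid index from 120-unit cells and the grid's N.
; The event graph has no active logic.
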(event EventBeginPlay)

(event Collision|EventActorBeginOverlap
  (params (OtherActor :type Actor%20Object%20Reference)))

(event EventTick
  (params (DeltaSeconds :type Float%20%28single-precision%29)))

(fn ConstructionScript
  (bind _returnvalue (Rendering|Material|CreateDynamicMaterialInstance (Variables|Default|GetPawn) 0 "/Game/Materials/M_OpponentPawn.M_OpponentPawn" :!class /Script/Engine.PrimitiveComponent))
  (Variables|Default|SetOpponentPawn_Material _returnvalue)
  (bind _outactors (Actor|GetAllActorsOfClass "/Game/Blueprints/BP_Amazon_GridMaster.BP_Amazon_GridMaster_C"))
  (Variables|Default|SetGridMaster (Utilities|Array|Get(acopy) _outactors)))