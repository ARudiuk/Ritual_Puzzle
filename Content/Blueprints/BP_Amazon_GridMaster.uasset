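; Grid manager for an Amazons-style board, holding the tile actors, the grid values and the possessed pawn index.
; Simple setters populate that state, with tiles registered one at a time through AddTile.
; GetMoveableTiles passes the grid, dimension N and pawn index to GetAmazonMoves, applies a slight glow to each resulting tile, and returns the move indices.
; Event graph and construction script are empty.
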(event EventActorBeginOverlap
  (params (OtherActor :type Actor%20Object%20Reference)))

(event EventTick
  (params (DeltaSeconds :type Float%20%28single-precision%29)))

(event EventBeginPlay)

(fn ConstructionScript)

(fn AddTile
  (params (Tile :type BP%20Amazon%20Grid%20Object%20Reference))
  (Utilities|Array|Add (Variables|Default|GetTile_List) Tile))

(fn SetGridValue
  (params (Unit :type Array%20of%20Integers))
  (Variables|Default|SetGrid Unit))

(fn GetMoveableTiles
  (bind _grid (Variables|Default|GetGrid))
  (for _array_element _grid
    _)
  (bind _returnvalue (Class|AmazonLevels|GetAmazonMoves _grid (Variables|Default|GetN) (Variables|Default|GetPossessed_Pawn_Index)))
  (for _array_element_2 _returnvalue
    (Default|SlightGlow (Utilities|Array|Get(acopy) (Variables|Default|GetTile_List) _array_element_2)))
  (return _returnvalue))

(fn SetPossessedPawnIndex
  (params (Index :type Integer))
  (Variables|Default|SetPossessed_Pawn_Index Index))