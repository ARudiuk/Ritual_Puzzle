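; BP_Amazon_Grid is a grid tile actor that glows when the cursor hovers over it.
; The construction script creates a dynamic instance of M_Amazon_Tile on the Tile component and stores it as TileMaterial.
; Cursor-over events drive that material's Glow parameter to full on hover and off on exit, while SlightGlow offers a half-strength highlight that nothing in this Blueprint calls.
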(event EventBeginPlay)

(event EventActorBeginOverlap
  (params (OtherActor :type Actor%20Object%20Reference)))

(event MouseInput|EventActorBeginCursorOver
  (Rendering|Material|SetScalarParameterValue (Variables|Default|GetTile_Material) "Glow" 1e+01 :!class /Script/Engine.MaterialInstanceDynamic))

(event MouseInput|EventActorEndCursorOver
  (Rendering|Material|SetScalarParameterValue (Variables|Default|GetTile_Material) "Glow" 0.0 :!class /Script/Engine.MaterialInstanceDynamic))

(event EventTick
  (params (DeltaSeconds :type Float%20%28single-precision%29)))

(fn ConstructionScript
  (bind _returnvalue (Rendering|Material|CreateDynamicMaterialInstance (Variables|Default|GetTile) 0 "/Game/Materials/M_Amazon_Tile.M_Amazon_Tile" :!class /Script/Engine.PrimitiveComponent))
  (Variables|Default|SetTile_Material _returnvalue))

(fn SlightGlow
  (Rendering|Material|SetScalarParameterValue (Variables|Default|GetTile_Material) "Glow" 5.0 :!class /Script/Engine.MaterialInstanceDynamic))